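; Main camera actor that follows a Target actor with smoothed movement and switchable zoom distance.
; BeginPlay stores the initial offset from the Target and enables player input.
; Each Tick, it interpolates toward the Target's position plus that offset times OffsetScale.
; The Action input cycles OffsetScale through a looping MultiGate, from directly on the Target to the original and doubled offsets.
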(event EventBeginPlay
  (Variables|Default|SetTargetOffset (- (Transformation|GetActorLocation) (Transformation|GetActorLocation (Variables|Parameters|GetTarget))))
  (Input|EnableInput (Game|GetPlayerController 0)))

(event EventTick
  (params (DeltaSeconds :type Float%20%28single-precision%29))
  (Transformation|SetActorLocation (Math|Interpolation|VInterpTo (Transformation|GetActorLocation) (+ (* (Variables|Default|GetTargetOffset) (Variables|Parameters|GetOffsetScale)) (Transformation|GetActorLocation (Variables|Parameters|GetTarget))) DeltaSeconds (Variables|Parameters|GetSpeed)) false false))

(event Input|ActionEvents|InputActionAction
  (params (Key :type Key%20Structure :default "AnyKey"))
  (:Pressed
    (Utilities|FlowControl|MultiGate false true -1
      (:Out%200
        (Variables|Parameters|SetOffsetScale 0.0))
      (:Out%201
        (Variables|Parameters|SetOffsetScale 1.0))
      (:Out%202
        (Variables|Parameters|SetOffsetScale 2.0)))))

(fn ConstructionScript)