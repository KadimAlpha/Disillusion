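; Coin-gated level exit: a gate that charges the third-person character a set number of coins to open, then leads to another level.
; Overlapping the actor checks the player's coins; with enough, it deducts the cost, deactivates trigger and text, activates Exit and sets Open.
; Exit's overlap event loads the configured level.
; The construction script attaches boxes to the gate-leaf sockets and writes the price on the text.
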(event Custom|Unlock%20Door
  (bind _player (Variables|Default|GetPlayer))
  (Variables|/Game/ThirdPersonBP/Blueprints/ThirdPersonCharacter.ThirdPersonCharacter_C|SetCoins _player (- (Variables|/Game/ThirdPersonBP/Blueprints/ThirdPersonCharacter.ThirdPersonCharacter_C|GetCoins _player) (Variables|Default|GetCoins)))
  (Components|Activation|Deactivate (Variables|Default|GetTrigger))
  (Components|Activation|Activate (Variables|Default|GetExit) false)
  (Components|Activation|Deactivate (Variables|Default|GetText))
  (Variables|Default|SetOpen true))

(event Custom|Check%20Coins
  (Math|Integer|CompareInt (Variables|/Game/ThirdPersonBP/Blueprints/ThirdPersonCharacter.ThirdPersonCharacter_C|GetCoins (Variables|Default|GetPlayer)) (Variables|Default|GetCoins)
    (:>
      _)
    (:==
      _))
  (CallFunction|UnlockDoor))

(event Custom|OnComponentBeginOverlap_Event_0
  (params (OverlappedComponent :type Primitive%20Component%20Object%20Reference) (OtherActor :type Actor%20Object%20Reference) (OtherComp :type Primitive%20Component%20Object%20Reference) (OtherBodyIndex :type Integer) (bFromSweep :type Boolean) (SweepResult :type Hit%20Result%20Structure%20%28by%20ref%29))
  (Game|OpenLevel(byName) (Variables|Default|GetLevel)))

(event Collision|EventActorBeginOverlap
  (params (OtherActor :type Actor%20Object%20Reference))
  (bind _asthird_person_character (Utilities|Casting|CastToThirdPersonCharacter OtherActor))
  (Variables|Default|SetPlayer _asthird_person_character)
  (CallFunction|CheckCoins))

(event EventBeginPlay
  (Collision|AssignOnComponentBeginOverlap (Variables|Default|GetExit) (delegate Custom|OnComponentBeginOverlap_Event_0))
  (Components|Activation|Deactivate (Variables|Default|GetExit)))

(fn ConstructionScript
  (Transformation|AttachComponentToComponent (Variables|Default|GetBox1) (Variables|Default|Getgate3_Gate_L) "Gate_L" "KeepRelative" "KeepRelative" "KeepRelative" true)
  (Transformation|AttachComponentToComponent (Variables|Default|GetBox) (Variables|Default|Getgate3_Gate_R) "Gate_R" "KeepRelative" "KeepRelative" "KeepRelative" true)
  (Rendering|Components|TextRender|SetText (Variables|Default|GetText) (Utilities|Text|ToText(String) (Utilities|String|Append "Coins: " (Utilities|String|ToString(Integer) (Variables|Default|GetCoins))))))

(fn NewFunction0)