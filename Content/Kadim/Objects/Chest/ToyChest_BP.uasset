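; Toy chest that the player opens once with the Use input while overlapping it, with a text prompt shown until then.
; Opening sets the first GohmCharacter's target to this chest and changes its state.
; After a delay, the chest spawns a pickup above itself and launches it forward and up with an impulse.
; The construction script tints the mesh through a dynamic material using the Color variable.
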(event Custom|Opened
  (if (not (Variables|Default|GetOpened?))
    (Variables|Default|SetOpened? true)
    (Rendering|SetVisibility (Variables|Default|GetTextRender) false false)
    (bind _outactors (Actor|GetAllActorsOfClass "/Game/Kadim/Characters/Sir_Gohm/AI/GohmCharacter.GohmCharacter_C"))
    (Default|SetTargetChest (Utilities|Array|Get(acopy) _outactors) self)
    (Default|UpdateState (Utilities|Array|Get(acopy) _outactors) "NewEnumerator9")
    (Utilities|FlowControl|Delay 2.6)
    (bind _returnvalue (Game|SpawnActorfromClass "/Game/Kadim/Prefabs/Pickup.Pickup_C" (Math|Transform|MakeTransform (+ (Transformation|GetActorLocation) "0.000000,0.000000,50.000000") (Transformation|GetActorRotation)) "Undefined" 0 0))
    (Physics|AddImpulse (Variables|/Game/Kadim/Prefabs/Pickup.Pickup_C|GetCollider _returnvalue) (+ (* "500.000000,500.000000,500.000000" (Math|Vector|GetForwardVector (Transformation|GetActorRotation))) "0, 0,200.000000") "None" true)))

(event Collision|EventActorBeginOverlap
  (params (OtherActor :type Actor%20Object%20Reference))
  (Utilities|Casting|CastToThirdPersonCharacter OtherActor)
  (Variables|Default|SetCanOpen true)
  (if (not (Variables|Default|GetOpened?))
    (Rendering|SetVisibility (Variables|Default|GetTextRender) true false)))

(event Collision|EventActorEndOverlap
  (params (OtherActor :type Actor%20Object%20Reference))
  (Utilities|Casting|CastToThirdPersonCharacter OtherActor)
  (Variables|Default|SetCanOpen false)
  (Rendering|SetVisibility (Variables|Default|GetTextRender) false false))

(event Input|ActionEvents|InputActionUse
  (params (Key :type Key%20Structure :default "AnyKey"))
  (:Pressed
    (if (Variables|Default|GetCanOpen)
      (CallFunction|Opened))))

(fn ConstructionScript
  (bind _returnvalue (Rendering|Material|CreateDynamicMaterialInstance (Variables|Default|GetSkeletalMesh) 0 "/Game/Kadim/Objects/Chest/ToyChest.ToyChest" :!class /Script/Engine.PrimitiveComponent))
  (Rendering|Material|SetVectorParameterValue _returnvalue "Color" (Variables|Default|GetColor) :!class /Script/Engine.MaterialInstanceDynamic))